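; Player controller for a rail shooter that possesses the primary character and fires the M4 of the active primary or secondary character.
; Left click fires once, or in Auto mode opens a Tick gate throttled by a short delay, blocked when crouched or out of ammo.
; Each shot plays sound, traces under the cursor for target-specific impact effects, spawns a muzzle projectile toward the hit and directly applies damage.
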(event EventBeginPlay
  (Pawn|Possess (Utilities|Array|Get(acopy) (Variables|/Game/BPMain/Interface/Ingame/BP_RailShootGameMode.BP_RailShootGameMode_C|GetPrimaryCH (.AsBP%20Rail%20Shoot%20Game%20Mode (Utilities|Casting|CastToBP_RailShootGameMode (Game|GetGameMode)))))))

(event EventTick
  (params (DeltaSeconds :type Float%20%28single-precision%29))
  (bind _returnvalue (Game|GetGameMode))
  (bind _array (Utilities|Array|MakeArray "ObjectTypeQuery1" "ObjectTypeQuery6"))
  (bind _hitresult (Class|PlayerController|GetHitResultUnderCursorforObjects _array true))
  (bind _asbp_rail_shoot_game_mode (Utilities|Casting|CastToBP_RailShootGameMode _returnvalue))
  (bind (_bblockinghit _binitialoverlap _time _distance _location _impactpoint _normal _impactnormal _physmat _hitactor) (Collision|BreakHitResult _hitresult))
  (bind _primarych (Variables|/Game/BPMain/Interface/Ingame/BP_RailShootGameMode.BP_RailShootGameMode_C|GetPrimaryCH _asbp_rail_shoot_game_mode))
  (bind _simpleai_1 (Variables|/Game/BPMain/Interface/Ingame/BP_RailShootGameMode.BP_RailShootGameMode_C|GetSimpleAI_1 _asbp_rail_shoot_game_mode))
  (bind _secondch (Variables|/Game/BPMain/Interface/Ingame/BP_RailShootGameMode.BP_RailShootGameMode_C|GetSecondCH _asbp_rail_shoot_game_mode))
  (bind _output (Utilities|Array|Get(acopy) _primarych))
  (bind _output_2 (Utilities|Array|Get(acopy) _secondch))
  (bind _m4 (Variables|/Game/BPMain/BP_PrimaryCH.BP_PrimaryCH_C|GetM4 _output))
  (bind _m4_2 (Variables|/Game/BPMain/BP_SecondCH.BP_SecondCH_C|GetM4 _output_2))
  (bind _returnvalue_2 (Transformation|GetSocketLocation _m4 "Muzzle"))
  (bind _returnvalue_3 (Transformation|GetSocketLocation _m4_2 "Muzzle"))
  (Utilities|FlowControl|Gate true
    (:Exit
      (if (Variables|Default|GetShootDelay)
        (Utilities|FlowControl|Delay 0.1)
        (Variables|Default|SetShootDelay false)
        (elif (Variables|/Game/BPMain/BP_PrimaryCH.BP_PrimaryCH_C|GetPosessFirst _output)
          (if (not (or (Variables|/Game/BPMain/BP_PrimaryCH.BP_PrimaryCH_C|GetCrouchTrue _output) (== (Variables|/Game/BPMain/BP_PrimaryCH.BP_PrimaryCH_C|GetAmmo _output) 0)))
            (Variables|Default|SetShootDelay true) ; engage delay for auto mode
            (Default|AmmoUpdate _output)
            (Audio|PlaySoundatLocation "/Game/BPMain/Resource/Sound/M4A1_Single-Kibblesbob-8540445.M4A1_Single-Kibblesbob-8540445" (Transformation|GetActorLocation) :!label _label) ; Play firing sound
            ;[1 1 1] 마우스 인식
            (if (== _hitactor _simpleai_1)
              ;[1 1 1] SimpleAI1/ Spawn Emitter at location
              (if (Variables|/Game/BPMain/ActorClass/SimpleAI.SimpleAI_C|GetCrouchAnimTrue _simpleai_1)
                (Effects|SpawnEmitteratLocation "/Game/InfinityBladeEffects/Effects/FX_Mobile/Impacts/P_Impact_Shield_Ice.P_Impact_Shield_Ice" _location "0, 0, 0" "0.500000,0.500000,0.500000")
                (else
                  (Effects|SpawnEmitteratLocation "/Game/BPMain/Resource/Particle/P_blood.P_blood" _location "0, 0, 0" "0.500000,0.500000,0.500000")))
              (else
                (Effects|SpawnEmitteratLocation "/Game/StarterContent/Particles/P_Explosion.P_Explosion" _location "0, 0, 0" "0.500000,0.500000,0.500000")))
            (if (Variables|/Game/BPMain/BP_PrimaryCH.BP_PrimaryCH_C|GetPosessFirst _output)
              (Game|SpawnActorfromClass "/Game/BPMain/ActorClass/BP_ProjectileEnemy.BP_ProjectileEnemy_C" (Math|Transform|MakeTransform _returnvalue_2 (Math|Rotator|FindLookatRotation _returnvalue_2 _location)) "Undefined" 0 0)
              (else
                (Game|SpawnActorfromClass "/Game/BPMain/ActorClass/BP_ProjectileEnemy.BP_ProjectileEnemy_C" (Math|Transform|MakeTransform _returnvalue_3 (Math|Rotator|FindLookatRotation _returnvalue_3 _location)) "Undefined" 0 0)))
            (Game|Damage|ApplyDamage _hitactor 5e+01 0 0))
          (elif (not (or (Variables|/Game/BPMain/BP_SecondCH.BP_SecondCH_C|GetCrouchTrue _output_2) (== (Variables|/Game/BPMain/BP_SecondCH.BP_SecondCH_C|GetAmmo _output_2) 0)))
            (Variables|Default|SetShootDelay true) ; engage delay for auto mode
            (Default|AmmoUpdate _output_2)
            (goto _label)))))))

(event Input|MouseEvents|LeftMouseButton
  (params (Key :type Key%20Structure))
  (bind _returnvalue (Game|GetGameMode))
  (bind _array (Utilities|Array|MakeArray "ObjectTypeQuery1" "ObjectTypeQuery6"))
  (bind _hitresult (Class|PlayerController|GetHitResultUnderCursorforObjects _array true))
  (bind _asbp_rail_shoot_game_mode (Utilities|Casting|CastToBP_RailShootGameMode _returnvalue))
  (bind (_bblockinghit _binitialoverlap _time _distance _location _impactpoint _normal _impactnormal _physmat _hitactor) (Collision|BreakHitResult _hitresult))
  (bind _primarych (Variables|/Game/BPMain/Interface/Ingame/BP_RailShootGameMode.BP_RailShootGameMode_C|GetPrimaryCH _asbp_rail_shoot_game_mode))
  (bind _simpleai_1 (Variables|/Game/BPMain/Interface/Ingame/BP_RailShootGameMode.BP_RailShootGameMode_C|GetSimpleAI_1 _asbp_rail_shoot_game_mode))
  (bind _secondch (Variables|/Game/BPMain/Interface/Ingame/BP_RailShootGameMode.BP_RailShootGameMode_C|GetSecondCH _asbp_rail_shoot_game_mode))
  (bind _output (Utilities|Array|Get(acopy) _primarych))
  (bind _output_2 (Utilities|Array|Get(acopy) _secondch))
  (bind _m4 (Variables|/Game/BPMain/BP_PrimaryCH.BP_PrimaryCH_C|GetM4 _output))
  (bind _m4_2 (Variables|/Game/BPMain/BP_SecondCH.BP_SecondCH_C|GetM4 _output_2))
  (bind _returnvalue_2 (Transformation|GetSocketLocation _m4 "Muzzle"))
  (bind _returnvalue_3 (Transformation|GetSocketLocation _m4_2 "Muzzle"))
  (:Pressed
    (if (Variables|Default|GetAuto)
      (Utilities|FlowControl|Gate true) ; enters at Open
      (elif (Variables|/Game/BPMain/BP_PrimaryCH.BP_PrimaryCH_C|GetPosessFirst _output)
        (if (not (or (Variables|/Game/BPMain/BP_PrimaryCH.BP_PrimaryCH_C|GetCrouchTrue _output) (== (Variables|/Game/BPMain/BP_PrimaryCH.BP_PrimaryCH_C|GetAmmo _output) 0)))
          (Variables|Default|SetShootDelay true) ; engage delay for auto mode
          (Default|AmmoUpdate _output)
          (Audio|PlaySoundatLocation "/Game/BPMain/Resource/Sound/M4A1_Single-Kibblesbob-8540445.M4A1_Single-Kibblesbob-8540445" (Transformation|GetActorLocation) :!label _label) ; Play firing sound
          ;[1 1 1] 마우스 인식
          (if (== _hitactor _simpleai_1)
            ;[1 1 1] SimpleAI1/ Spawn Emitter at location
            (if (Variables|/Game/BPMain/ActorClass/SimpleAI.SimpleAI_C|GetCrouchAnimTrue _simpleai_1)
              (Effects|SpawnEmitteratLocation "/Game/InfinityBladeEffects/Effects/FX_Mobile/Impacts/P_Impact_Shield_Ice.P_Impact_Shield_Ice" _location "0, 0, 0" "0.500000,0.500000,0.500000")
              (else
                (Effects|SpawnEmitteratLocation "/Game/BPMain/Resource/Particle/P_blood.P_blood" _location "0, 0, 0" "0.500000,0.500000,0.500000")))
            (else
              (Effects|SpawnEmitteratLocation "/Game/StarterContent/Particles/P_Explosion.P_Explosion" _location "0, 0, 0" "0.500000,0.500000,0.500000")))
          (if (Variables|/Game/BPMain/BP_PrimaryCH.BP_PrimaryCH_C|GetPosessFirst _output)
            (Game|SpawnActorfromClass "/Game/BPMain/ActorClass/BP_ProjectileEnemy.BP_ProjectileEnemy_C" (Math|Transform|MakeTransform _returnvalue_2 (Math|Rotator|FindLookatRotation _returnvalue_2 _location)) "Undefined" 0 0)
            (else
              (Game|SpawnActorfromClass "/Game/BPMain/ActorClass/BP_ProjectileEnemy.BP_ProjectileEnemy_C" (Math|Transform|MakeTransform _returnvalue_3 (Math|Rotator|FindLookatRotation _returnvalue_3 _location)) "Undefined" 0 0)))
          (Game|Damage|ApplyDamage _hitactor 5e+01 0 0))
        (elif (not (or (Variables|/Game/BPMain/BP_SecondCH.BP_SecondCH_C|GetCrouchTrue _output_2) (== (Variables|/Game/BPMain/BP_SecondCH.BP_SecondCH_C|GetAmmo _output_2) 0)))
          (Variables|Default|SetShootDelay true) ; engage delay for auto mode
          (Default|AmmoUpdate _output_2)
          (goto _label)))))
  (:Released
    (Utilities|FlowControl|Gate true) ; enters at Close
  ))

(fn ConstructionScript)